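; A cine camera actor that serves as the shared game camera for a two-player game.
; On BeginPlay, after a short delay, it caches both player references from the default game mode and becomes the first player controller's view target.
; Tick is empty; disconnected leftover logic would move the camera between the players, scale field of view by their separation, and set the second controller's view, but none of it runs.
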(event `self.ReceiveTick`
  (params (DeltaSeconds :type "Float (single-precision)")))

(event `self.ReceiveBeginPlay`
  (`KismetSystemLibrary.Delay` 0.5)
  (bind _asgame_mode_bp_default_game_mode_base (cast `/Game/Blueprints/GameMode/GameMode_BP_DefaultGameModeBase` (`GameplayStatics.GetGameMode`)))
  (set `self.Player 1Ref` (`FighterGameModeBase.Player1Ref` _asgame_mode_bp_default_game_mode_base))
  (set `self.Player 2Ref` (`FighterGameModeBase.Player2Ref` _asgame_mode_bp_default_game_mode_base))
  (`PlayerController.SetViewTargetWithBlend` (`GameplayStatics.GetPlayerController` 0) self 0.0 "VTBlend_Linear" 0.0 false))

(fn `UserConstructionScript`)