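; BP_AICharacter is an AI-driven fighter character that chases and attacks another fighter.
; Each Tick, while its AI controller is valid and HealthComp reports it alive, it measures the distance to OtherFighter.
; Beyond a fixed range it moves toward that fighter via the AI controller with navmesh projection.
; Within range it stops movement and feeds simulated button input into AttackStateMachineComponent.
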(event `self.ReceiveBeginPlay`)

(event `self.ReceiveTick`
  (params (DeltaSeconds :type "Float (single-precision)"))
  (bind _attackstatemachinecomponent (`self.AttackStateMachineComponent`))
  (`/Engine/EditorBlueprintResources/StandardMacros.IsValid` (`AIBlueprintHelperLibrary.GetAIController` self)
    (:`Is Valid`
      (bind _returnvalue (`HealthComponent.IsActorAlive` (`self.HealthComp`) self))
      (if _returnvalue
        (if (> (`KismetMathLibrary.Vector_Distance` (`self.K2_GetActorLocation` (`self.OtherFighter`)) (`self.K2_GetActorLocation`)) 250.0)
          (`AIController.MoveToLocation` (`AIBlueprintHelperLibrary.GetAIController` self) (`self.K2_GetActorLocation` (`self.OtherFighter`)) 10.0 true true true true null true)
          (else
            (`NavMovementComponent.StopActiveMovement` (`self.CharacterMovement`))
            (`AttackStateMachine.SetInputButton` _attackstatemachinecomponent 1)
            (`AttackStateMachine.SetInputState` _attackstatemachinecomponent 1)))))))

(fn `UserConstructionScript`)