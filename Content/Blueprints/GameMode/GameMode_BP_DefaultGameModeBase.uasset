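; Base game mode that spawns and pairs the two fighters of a versus match at BeginPlay.
; It loops over PlayerStarts by tag, spawning a test character possessed by the first player controller at P1 and an AI character at P2.
; When both exist, it links each as the other's opponent and flips the second fighter.
; A second-controller possess node is left unconnected.
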(event `self.ReceiveBeginPlay`
  (bind _player2ref (`self.Player2Ref`))
  (bind _outactors (`GameplayStatics.GetAllActorsOfClass` "/Script/Engine.PlayerStart"))
  (for _array_element _outactors
    (`self.SpawnPlayersOnSpawnPoint` _array_element))
  (if (`KismetSystemLibrary.IsValid` (`self.Player1Ref`))
    (if (`KismetSystemLibrary.IsValid` (`self.Player2Ref`))
      (`BaseSideFighterCharacter.SetOtherFighter` (`self.Player1Ref`) (`self.Player2Ref`))
      (`BaseSideFighterCharacter.SetOtherFighter` _player2ref (`self.Player1Ref`))
      (set `BaseSideFighterCharacter.isFlipped` true _player2ref))))

(fn `SpawnPlayersOnSpawnPoint`
  (params (PlayerStart :type "PlayerStart Object Reference"))
  (`/Engine/EditorBlueprintResources/StandardMacros.IsValid` PlayerStart
    (:`Is Valid`
      (if (== "P1" (`PlayerStart.PlayerStartTag` PlayerStart))
        (bind _returnvalue (`|SpawnActorFromClass` "/Game/Blueprints/Characters/TestCharacter/BP_TestCharacter.BP_TestCharacter_C" (`self.GetTransform` PlayerStart) "Undefined" "OverrideRootScale" PlayerStart null))
        (set `self.Player1Ref` _returnvalue)
        (`Controller.Possess` (`GameplayStatics.GetPlayerController` 0) _returnvalue)
        (elif (== "P2" (`PlayerStart.PlayerStartTag` PlayerStart))
          (bind _returnvalue_2 (`|SpawnActorFromClass` "/Game/Blueprints/Characters/TestCharacter/BP_AICharacter.BP_AICharacter_C" (`self.GetTransform` PlayerStart) "Undefined" "OverrideRootScale" PlayerStart null))
          (set `self.Player2Ref` _returnvalue_2))))))

(fn `UserConstructionScript`)